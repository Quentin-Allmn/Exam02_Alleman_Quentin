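; BP_Spell is a short-lived spell actor that damages enemies and destroys itself three seconds after spawning.
; Each Tick it line traces on Visibility from its Sphere to the scaled forward vector, which is used as a world position without adding the start location.
; A hit BP_Enemies takes Damage and an impact particle spawns at the hit point.
; The spell persists after hits, so damage can repeat every frame.
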(event EventBeginPlay
  (Utilities|FlowControl|Delay 3.0)
  (Actor|DestroyActor))

(event Collision|EventActorBeginOverlap
  (params (OtherActor :type Actor%20Object%20Reference)))

(event EventTick
  (params (DeltaSeconds :type Float%20%28single-precision%29))
  (bind _sphere (Variables|Default|GetSphere))
  ;[1 1 1] Enemy Detection
  (bind _outhit (Collision|LineTraceByChannel (Transformation|GetWorldLocation _sphere) (* (Math|Vector|GetForwardVector (Transformation|GetWorldRotation _sphere)) 3e+02) "TraceTypeQuery1" false 0 "None"))
  (bind _asbp_enemies (Utilities|Casting|CastToBP_Enemies (.HitActor (Collision|BreakHitResult _outhit))))
  (Default|TakeDamage _asbp_enemies (Variables|Default|GetDamage))
  (Effects|SpawnEmitteratLocation "/Game/VFX/PolygonPirates/ParticleFX/P_FX_SpellImpact.P_FX_SpellImpact" (.ImpactPoint (Collision|BreakHitResult _outhit))))

(fn ConstructionScript)