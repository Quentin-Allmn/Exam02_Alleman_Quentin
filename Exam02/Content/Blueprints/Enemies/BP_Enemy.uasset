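; BP_Enemy is a skeleton swordsman enemy that plays an attack when its line of sight hits the player.
; Each Tick it traces the Visibility channel from its capsule to the root's forward vector times a range, without adding the start location.
; A BP_Player hit plays the attack montage, with IsAttacking blocking retriggers until it completes.
; BeginPlay initializes PV, which is not otherwise used here.
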(event EventBeginPlay
  (Variables|Default|SetPV 1.5e+02))

(event Collision|EventActorBeginOverlap
  (params (OtherActor :type Actor%20Object%20Reference)))

(event EventTick
  (params (DeltaSeconds :type Float%20%28single-precision%29))
  (bind _outhit (Collision|LineTraceByChannel (Transformation|GetWorldLocation (Variables|Default|GetCapsule)) (* (Math|Vector|GetForwardVector (Transformation|GetWorldRotation (Variables|Default|GetDefaultSceneRoot))) 1.5e+03) "TraceTypeQuery1" false 0 "None"))
  (Utilities|Casting|CastToBP_Player (.HitActor (Collision|BreakHitResult _outhit)))
  (if (not (Variables|Default|GetIs%20Attacking))
    (Variables|Default|SetIs%20Attacking true)
    (Animation|Montage|PlayMontage 0 "/Game/SkeletonCrew/Skeleton_Swordman/Animations/Skeleton_Swordman_Default_Attack_Montage.Skeleton_Swordman_Default_Attack_Montage"
      (:OnCompleted
        (Variables|Default|SetIs%20Attacking false)))))

(fn ConstructionScript)