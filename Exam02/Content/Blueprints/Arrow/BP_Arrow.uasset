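; BP_Arrow is an arrow actor that damages the player and destroys itself three seconds after spawning.
; Each Tick it runs an undrawn Visibility line trace from the Cube's location to its forward vector times 300, without adding the start location.
; A BP_Player hit takes damage and triggers an emitter spawn; the arrow is not destroyed on hit, so this can repeat every frame.
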(event EventBeginPlay
  (Utilities|FlowControl|Delay 3.0)
  (Actor|DestroyActor))

(event Collision|EventActorBeginOverlap
  (params (OtherActor :type Actor%20Object%20Reference)))

(event EventTick
  (params (DeltaSeconds :type Float%20%28single-precision%29))
  (bind _cube (Variables|Default|GetCube))
  ;[1 1 1] Enemy Detection
  (bind _outhit (Collision|LineTraceByChannel (Transformation|GetWorldLocation _cube) (* (Math|Vector|GetForwardVector (Transformation|GetWorldRotation _cube)) 3e+02) "TraceTypeQuery1" false 0 "None"))
  (bind _asbp_player (Utilities|Casting|CastToBP_Player (.HitActor (Collision|BreakHitResult _outhit))))
  (Default|TakeDamage _asbp_player (Variables|Default|Getdamage))
  (Effects|SpawnEmitteratLocation 0 "0, 0, 0"))

(fn ConstructionScript)